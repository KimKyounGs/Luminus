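; BP_Projectil_Base is a projectile, filed under AI, that flies at a set speed and gravity toward an optional target, with optional homing.
; The construction script configures ProjectileMovement, including homing on the target's root component.
; BeginPlay ignores the owner for box collision movement and aims velocity at any valid target.
; On hit, it broadcasts OnProjectilImpact with actor and hit data, spawns impact effect and sound, then destroys itself.
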(event OnComponentHit(BoxCollision)
  (params (HitComponent :type Primitive%20Component%20Object%20Reference) (OtherActor :type Actor%20Object%20Reference) (OtherComp :type Primitive%20Component%20Object%20Reference) (NormalImpulse :type Vector :default "0, 0, 0") (Hit :type Hit%20Result%20Structure%20%28by%20ref%29))
  (bind _location (Collision|BreakHitResult Hit))
  (Default|CallOnProjectilImpact OtherActor Hit)
  (Effects|SpawnEmitteratLocation (Variables|ProjectilSettings|GetImpactEffect) _location)
  (Audio|PlaySoundatLocation (Variables|ProjectilSettings|GetImpactSound) _location "0, 0, 0" 1.0 1.0 0.0 0 0 0 0)
  (Actor|DestroyActor))

(event Custom|RotateToTarget
  (Variables|/Script/Engine.MovementComponent|SetVelocity (Variables|Default|GetProjectileMovement) (* (Math|Vector|GetUnitDirection(Vector) (Transformation|GetActorLocation) (Transformation|GetActorLocation (Variables|타깃|GetTarget))) (Variables|ProjectilSettings|GetSpeed))))

(event EventBeginPlay
  (Collision|IgnoreActorwhenMoving (Variables|Default|GetBoxCollision) (Components|GetOwner) true)
  (Variables|타깃|GetTarget
    (:then
      (CallFunction|RotatetoTarget))
    (:else)))

(event Collision|EventActorBeginOverlap
  (params (OtherActor :type Actor%20Object%20Reference)))

(event EventTick
  (params (DeltaSeconds :type Float%20%28single-precision%29)))

(fn ConstructionScript
  (bind _projectilemovement (Variables|Default|GetProjectileMovement))
  (Variables|/Script/Engine.ProjectileMovementComponent|SetInitialSpeed _projectilemovement (Variables|ProjectilSettings|GetSpeed))
  (Variables|/Script/Engine.ProjectileMovementComponent|SetMaxSpeed _projectilemovement (Variables|ProjectilSettings|GetSpeed))
  (Variables|/Script/Engine.ProjectileMovementComponent|SetProjectileGravityScale _projectilemovement (Variables|ProjectilSettings|GetGravity))
  (Variables|타깃|GetTarget
    (:then
      (if (Variables|ProjectilSettings|GetIsHoming)
        (Variables|/Script/Engine.ProjectileMovementComponent|SetbIsHomingProjectile _projectilemovement true)
        (Variables|/Script/Engine.ProjectileMovementComponent|SetHomingTargetComponent _projectilemovement (Variables|/Script/Engine.Actor|GetRootComponent (Variables|타깃|GetTarget)))))
    (:else)))