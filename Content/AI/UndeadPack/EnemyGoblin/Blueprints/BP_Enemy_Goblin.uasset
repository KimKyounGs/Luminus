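; Goblin enemy Blueprint with a basic montage-driven melee attack.
; A custom event plays the attack montage on the mesh, applies damage as soon as playback starts with no target shown, and prints a debug message.
; Montage completion or interruption calls OnAttackEnd.
; Weapon equip events and functions for ideal range, movement speed and patrol route are stubs that are empty or return zero.
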(event Custom|CustomEvent
  (Animation|Montage|PlayMontage (Variables|Character|GetMesh) "/Game/AI/UndeadPack/EnemyGoblin/Animations/Goblin_Attack1_Montage.Goblin_Attack1_Montage"
    (:then
      (Game|Damage|ApplyDamage 0 1e+01 0 0)
      (Development|PrintText "Apply Damage"))
    (:OnCompleted
      (Default|CallOnAttackEnd :!label _label))
    (:OnInterrupted
      (goto _label))))

(event EventUnequipWeapon)

(event EventEquipWeapon)

(fn ConstructionScript
  (|CallParentFunction))

(fn GetIdealRange
  (return 0.0 0.0))

(fn SetMovementSpeed
  (params (Speed :type E_MovementSpeed%20Enum :default "NewEnumerator0"))
  (return 0.0))

(fn GetPatrolRoute
  (return 0))