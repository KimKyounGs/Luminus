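; Attack component for enemy AI that deals damage through hitscan bullets and magic projectiles.
; FireBullet line-traces for pawns, while MagicSpell spawns a targeted projectile that ignores its owner and fires OnAttackEnded on impact.
; Both send damage through a TakeDamage interface message and report it to AI damage sense.
; Team-filtered helpers damage the first non-team hit or track damaged actors to avoid repeats, though the latter's loop is disconnected.
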(event Custom|MagicSpell
  (params (SpawnTrasnform :type Transform) (Target :type Actor%20Object%20Reference) (DamageInfo :type S%20Damage%20Info%20Structure))
  (bind _returnvalue (Game|SpawnActorfromClass "/Game/AI/Projectile/BP_Projectil_Base_Prime.BP_Projectil_Base_Prime_C" SpawnTrasnform "Undefined" "MultiplyWithRoot" (Components|GetOwner) 5e+02 0.0 Target 0))
  (EventDispatchers|AssignOnProjectilImpact _returnvalue (delegate Custom|OnProjectileHit))
  (Collision|IgnoreActorwhenMoving (Variables|/Game/AI/Projectile/BP_Projectil_Base.BP_Projectil_Base_C|GetBoxCollision _returnvalue) (Components|GetOwner) true))

(event Custom|OnProjectileHit
  (params (Other%20Actor :type Actor%20Object%20Reference) (Hit :type Hit%20Result%20Structure))
  (bind _returnvalue (Components|GetOwner))
  (Class|BPIDamagalbe|TakeDamage(Message) Other%20Actor (stale Custom|MagicSpell DamageInfo) _returnvalue)
  (Class|AISenseDamage|ReportDamageEvent Other%20Actor _returnvalue (Utilities|Struct|BreakS_DamageInfo (stale Custom|MagicSpell DamageInfo)) (Transformation|GetActorLocation (Components|GetOwner)) "0, 0, 0" "None")
  (Default|CallOnAttackEnded))

(event Custom|FireBullet
  (params (TraceStart :type Vector) (TraceEnd :type Vector) (DamageInfo :type S%20Damage%20Info%20Structure))
  (bind (_outhit _returnvalue) (Collision|LineTraceForObjects TraceStart TraceEnd (Utilities|Array|MakeArray "ObjectTypeQuery3") false 0 "None"))
  (if _returnvalue
    (Class|BPIDamagalbe|TakeDamage(Message) (.HitActor (Collision|BreakHitResult _outhit)) DamageInfo)
    (Class|AISenseDamage|ReportDamageEvent (.HitActor (Collision|BreakHitResult _outhit)) (Components|GetOwner) (Utilities|Struct|BreakS_DamageInfo DamageInfo) (Transformation|GetActorLocation (Components|GetOwner)) "0, 0, 0" "None")))

(event EventBeginPlay)

(event EventTick
  (params (DeltaSeconds :type Float%20%28single-precision%29)))

(fn DamageAllNonTeamMembers
  (params (Hits :type Array%20of%20Hit%20Result%20Structures) (DamageInfo :type S%20Damage%20Info%20Structure))
  (bind _teamnumber (Class|BPIDamagalbe|GetTeamNumber(Message) (.HitActor (Collision|BreakHitResult (stale _array_element)))))
  (bind _teamnumber_2 (Class|BPIDamagalbe|GetTeamNumber(Message) (Components|GetOwner)))
  (if (and (!= _teamnumber_2 _teamnumber) (not (Utilities|Array|ContainsItem (LocalVariables|GetActorsDamagedSoFar) (.HitActor (Collision|BreakHitResult (stale _array_element))))))
    (Class|BPIDamagalbe|TakeDamage(Message) (.HitActor (Collision|BreakHitResult (stale _array_element))) DamageInfo (Components|GetOwner))
    ;[1 1 1] 이것을 이용해서 한명에게 한번의 데미지만 들어가게끔 함.
    (Utilities|Array|AddUnique (LocalVariables|GetActorsDamagedSoFar) (.HitActor (Collision|BreakHitResult (stale _array_element))))))

(fn DamagedFirstNonTeamMember
  (params (Hits :type Array%20of%20Hit%20Result%20Structures) (DamagedInfro :type S%20Damage%20Info%20Structure))
  (bind _array_element (Utilities|Array|ForEachLoopwithBreak Hits :!label _label)
    (:LoopBody
      (bind _teamnumber (Class|BPIDamagalbe|GetTeamNumber(Message) (.HitActor (Collision|BreakHitResult _array_element))))
      (bind _teamnumber_2 (Class|BPIDamagalbe|GetTeamNumber(Message) (Components|GetOwner)))
      (if (!= _teamnumber_2 _teamnumber)
        (Class|BPIDamagalbe|TakeDamage(Message) (.HitActor (Collision|BreakHitResult _array_element)) DamagedInfro (Components|GetOwner))
        (Utilities|FlowControl|Sequence
          (:then_0
            (goto _label Break))
          (:then_1
            (return (.HitActor (Collision|BreakHitResult _array_element)))))))))