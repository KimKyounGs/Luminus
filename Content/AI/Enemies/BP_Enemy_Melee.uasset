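; Melee enemy AI character that fights with a sword and supplies movement speeds, combat ranges and a patrol route.
; Attack plays an uninterruptible great-sword montage whose notify sphere-traces forward to deal damage, then signals attack end.
; A sword spawns at BeginPlay; equip and unequip also spawn or destroy one through montage notifies, firing event dispatchers.
; The construction script makes modular body meshes follow the main mesh's pose.
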(event Custom|SwordAttach
  (bind _returnvalue (Game|SpawnActorfromClass "/Game/AI/Enemies/BehaviorTrees/BP_Weapon_Sword.BP_Weapon_Sword_C" (Transformation|GetActorTransform) "Undefined" "MultiplyWithRoot" 0 0))
  (Transformation|AttachComponentToComponent _returnvalue (Variables|Character|GetMesh) "Enemy1Weapon_r" "SnapToTarget" "SnapToTarget" "SnapToTarget" true))

(event EventBeginPlay
  (CallFunction|SwordAttach)
  (|CallParentFunction))

(event Collision|EventActorBeginOverlap
  (params (OtherActor :type Actor%20Object%20Reference))
  (|CallParentFunction OtherActor) ; 지금 이 노드는 비활성 상태입니다. \n핀을 끌어서 다른 노드를 연결하면 활성화됩니다.
)

(event EventUnEquipWeapon
  ;[1 1 1] SheatSword
  (bind _notifyname (Animation|Montage|PlayMontage (Variables|Character|GetMesh) 0)
    (:OnCompleted
      (Default|CallOnWeaponUnEquipped))
    (:OnNotifyEnd
      (switch name _notifyname
        (:DropSword
          (Actor|DestroyActor (Variables|Default|GetWeaponActor))
          (Variables|Default|SetIsWieldingWeapon false))))))

(event EventEquipWeapon
  ;[1 1 1] WieldSword
  (Variables|Default|SetIsWieldingWeapon true)
  (bind _notifyname (Animation|Montage|PlayMontage (Variables|Character|GetMesh) 0)
    (:OnNotifyBegin
      (switch name _notifyname
        (:HoldSword
          (bind _returnvalue (Game|SpawnActorfromClass "/Game/AI/Enemies/BehaviorTrees/BP_Weapon_Sword.BP_Weapon_Sword_C" (Transformation|GetActorTransform) "Undefined" "MultiplyWithRoot" 0 0))
          (bind _output_get (Variables|Default|SetWeaponActor _returnvalue))
          (Transformation|AttachComponentToComponent _output_get (Variables|Character|GetMesh) "Enemy1Weapon_r" "SnapToTarget" "SnapToTarget" "SnapToTarget" true)
          (Default|CallOnWeaponEquipped))))))

(event EventAttack
  (bind _returnvalue (Transformation|GetActorLocation))
  ;[1 1 1] Attack
  (bind _notifyname (Animation|Montage|PlayMontage (Variables|Character|GetMesh) "/Game/AI/enemy_meta1/Animation/Great_Sword_Slash_Montage.Great_Sword_Slash_Montage")
    (:then
      (Variables|/Game/AI/Enemies/Damage/BPC_DamageSystem.BPC_DamageSystem_C|SetIsInterruptible (Variables|Default|GetBPC_DamageSystem) false))
    (:OnCompleted
      (Default|CallOnAttackEnd :!label _label)
      (Variables|/Game/AI/Enemies/Damage/BPC_DamageSystem.BPC_DamageSystem_C|SetIsInterruptible (Variables|Default|GetBPC_DamageSystem) true))
    (:OnInterrupted
      (goto _label))
    (:OnNotifyBegin
      (switch name _notifyname
        (:Slash
          (bind (_outhit _returnvalue_2) (Collision|SphereTraceForObjects _returnvalue (+ _returnvalue (* (Transformation|GetActorForwardVector) 2e+02)) 2e+01 (Utilities|Array|MakeArray "ObjectTypeQuery3") false 0 "ForDuration"))
          (if _returnvalue_2
            (Class|BPIDamagalbe|TakeDamage(Message) (.HitActor (Collision|BreakHitResult _outhit)) (Utilities|Struct|MakeS_DamageInfo 25.0 "NewEnumerator1") self)))))))

(fn ConstructionScript
  (|CallParentFunction)
  (Components|SkinnedMesh|SetLeaderPoseComponent (Variables|Default|GetTorso) (Variables|Character|GetMesh) false false))

(fn SetMovementSpeed
  (params (Speed :type E_MovementSpeed%20Enum :default "NewEnumerator0"))
  (bind _output_get (Variables|/Script/Engine.CharacterMovementComponent|SetMaxWalkSpeed (Variables|Character|GetCharacterMovement) (Utilities|Select :Index Speed :NewEnumerator0 0.0 :NewEnumerator1 1.5e+02 :NewEnumerator2 3e+02 :NewEnumerator3 5e+02)))
  (return _output_get))

(fn GetIdelRange
  (return 1.5e+02 3e+02))

(fn GetPatrolRoute
  (return (Variables|Default|GetBP_PatrolRoute)))