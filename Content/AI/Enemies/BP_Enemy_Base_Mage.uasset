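; Mage enemy Blueprint that attacks a target by casting a damaging magic spell during a montage.
; Attack plays the montage on the mesh, and its notify fires MagicSpell on the BPCAttacks component from the RightHand socket toward the target.
; AttackEnd runs whether the montage completes or is interrupted.
; Helper functions supply the mage's speed for each movement state and its attack and defend radii.
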(event EventBeginPlay
  (|CallParentFunction) ; 지금 이 노드는 비활성 상태입니다. \n핀을 끌어서 다른 노드를 연결하면 활성화됩니다.
)

(event Collision|EventActorBeginOverlap
  (params (OtherActor :type Actor%20Object%20Reference)))

(event EventTick
  (params (DeltaSeconds :type Float%20%28single-precision%29)))

(event EventAttack
  (params (AttackTarget :type Actor%20Object%20Reference))
  (bind _notifyname (Animation|Montage|PlayMontage (Variables|Character|GetMesh) 0)
    (:OnCompleted
      (CallFunction|AttackEnd AttackTarget :!label _label))
    (:OnInterrupted
      (goto _label))
    (:OnNotifyBegin
      (switch name _notifyname
        (:Fire
          (Default|MagicSpell (Variables|Default|GetBPC_Attacks) (Math|Transform|MakeTransform (Transformation|GetSocketLocation (Variables|Character|GetMesh) "RightHand") "0, 0, 0" "1.000000,1.000000,1.000000") AttackTarget (Utilities|Struct|MakeS_DamageInfo 2e+01 "NewEnumerator2" "NewEnumerator1")))))))

(fn ConstructionScript
  (|CallParentFunction))

(fn SetMovementSpeed
  (params (Speed :type E_MovementSpeed%20Enum :default "NewEnumerator0"))
  (return (Utilities|Select :Index Speed :NewEnumerator0 0.0 :NewEnumerator1 1.5e+02 :NewEnumerator2 2.5e+02 :NewEnumerator3 4e+02)))

(fn GetIdelRange
  (return 5e+02 7e+02))