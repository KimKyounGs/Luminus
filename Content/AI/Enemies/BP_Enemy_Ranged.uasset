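; Ranged enemy AI character Blueprint that supplies its attack behavior, attack and defend radius, movement speeds and patrol route.
; Attack plays a montage whose notify line-traces on Visibility from the weapon to the AI controller's attack target, printing "Hit" when unobstructed, with no damage applied.
; Montage completion or interruption signals attack end.
; Weapon equip and unequip events are empty stubs.
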(event EventBeginPlay
  (|CallParentFunction) ; 지금 이 노드는 비활성 상태입니다. \n핀을 끌어서 다른 노드를 연결하면 활성화됩니다.
)

(event Collision|EventActorBeginOverlap
  (params (OtherActor :type Actor%20Object%20Reference))
  (|CallParentFunction OtherActor) ; 지금 이 노드는 비활성 상태입니다. \n핀을 끌어서 다른 노드를 연결하면 활성화됩니다.
)

(event EventTick
  (params (DeltaSeconds :type Float%20%28single-precision%29))
  (|CallParentFunction DeltaSeconds) ; 지금 이 노드는 비활성 상태입니다. \n핀을 끌어서 다른 노드를 연결하면 활성화됩니다.
)

(event EventAttack
  (bind _notifyname (Animation|Montage|PlayMontage (Variables|Character|GetMesh) 0)
    (:OnCompleted
      (Default|CallOnAttackEnd :!label _label))
    (:OnInterrupted
      (goto _label))
    (:OnNotifyBegin
      (switch name _notifyname
        (:Default
          (bind _astest_aic_enemy_base (Utilities|Casting|CastToTest_AIC_Enemy_Base (AI|GetAIController self)))
          (bind _attacktarget (Variables|/Game/AI/Enemies/Test_AIC_Enemy_Base.Test_AIC_Enemy_Base_C|GetAttackTarget _astest_aic_enemy_base)
            (:then
              (bind _returnvalue (Collision|LineTraceByChannel (Transformation|GetActorLocation (Variables|Default|GetWeaponActor)) (Transformation|GetActorLocation _attacktarget) "TraceTypeQuery1" false 0 "ForDuration"))
              (if (not _returnvalue)
                (Development|PrintString "Hit")))
            (:else)))))))

(event EventUnEquipWeapon)

(event EventEquipWeapon)

(fn ConstructionScript
  (|CallParentFunction))

(fn GetIdelRange
  (return 6e+02 6e+02))

(fn SetMovementSpeed
  (params (Speed :type E_MovementSpeed%20Enum :default "NewEnumerator0"))
  (bind _output_get (Variables|/Script/Engine.CharacterMovementComponent|SetMaxWalkSpeed (Variables|Character|GetCharacterMovement) (Utilities|Select :Index Speed :NewEnumerator0 0.0 :NewEnumerator1 2e+02 :NewEnumerator2 3e+02 :NewEnumerator3 5e+02)))
  (return _output_get))

(fn GetPatrolRoute
  (return (Variables|Default|GetBP_PatrolRoute)))