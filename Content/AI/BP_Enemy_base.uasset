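; Base enemy character Blueprint providing attack, roaming and movement helpers for AI-driven enemies.
; Attack plays a goblin montage, calls ApplyDamage as playback starts with no target wired, and fires OnAttackEnd on completion or interruption.
; RoamAround moves to random reachable points, re-calling itself only after success.
; Functions expose combat ranges, a patrol route and enum-based walk speed, while weapon events and hit direction are empty stubs.
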(event Custom|Roam%20Around
  ;[1 1 1] Roam Around
  (AI|AIMoveTo self (.RandomLocation (AI|Navigation|GetRandomReachablePointinRadius (Transformation|GetActorLocation) 2e+03 0 0)) 0 1.2e+02 false
    (:OnSuccess
      (Utilities|FlowControl|Delay 0.2)
      (CallFunction|RoamAround))))

(event Custom|Attack
  (Animation|Montage|PlayMontage (Variables|Character|GetMesh) "/Game/AI/UndeadPack/EnemyGoblin/Animations/Goblin_Attack1_Montage.Goblin_Attack1_Montage"
    (:then
      (Game|Damage|ApplyDamage 0 1e+01 0 0)
      (Development|PrintText "Apply Damage"))
    (:OnCompleted
      (Default|CallOnAttackEnd :!label _label))
    (:OnInterrupted
      (goto _label))))

(event EventBeginPlay)

(event Collision|EventActorBeginOverlap
  (params (OtherActor :type Actor%20Object%20Reference)))

(event EventTick
  (params (DeltaSeconds :type Float%20%28single-precision%29)))

(event EventEquipWeapon
  ;[1 1 1] 무기를 껴야하는 상황이면 이 노드 사용하기.
)

(event EventUnequipWeapon
  ;[1 1 1] 무기를 껴야하는 상황이면 이 노드 사용하기.
)

(fn ConstructionScript)

(fn GetHitDirection
  (params (NewParam :type Boolean)))

(fn GetIdealRange
  (return 1.5e+02 3.5e+02))

(fn GetPatrolRoute
  (return (Variables|AI|GetPatrolRoute)))

(fn SetMovementSpeed
  (params (Speed :type E_MovementSpeed%20Enum :default "NewEnumerator0"))
  (bind _output_get (Variables|/Script/Engine.CharacterMovementComponent|SetMaxWalkSpeed (Variables|Character|GetCharacterMovement) (Utilities|Select :Index Speed :NewEnumerator0 0.0 :NewEnumerator1 1e+02 :NewEnumerator2 3e+02 :NewEnumerator3 5e+02)))
  (return _output_get))