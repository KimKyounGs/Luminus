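; Player character for sword combat, with combo attacks, rolling, a running mode that hides the sword, and guarding.
; Number keys select one of four four-hit montage combos; AttackSave plays buffered input and ResetCombo clears the chain.
; Flags gate actions, DoOnce plus montage-length delays lock roll and run toggles, and guard only draws a debug arc.
; Damage plays directional hit montages using dot/cross angles, and body-part meshes follow the main mesh's pose.
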(event Custom|AttackSave
  ;[1 1 1] Attack
  (if (not (Math|Boolean|ORBoolean (Variables|Default|GetIsFalling) (Variables|Default|GetIs%20Rolling) (Variables|Default|GetIs%20Running)))
    (if (Variables|Default|GetSave%20Attack)
      (Variables|Default|SetSave%20Attack false)
      (switch int (Variables|Default|GetAttack%20Type)
        (:0
          (switch int (Variables|Default|GetAttack%20Count)
            (:0
              (Variables|Default|SetAttack%20Count 1)
              (Animation|PlayAnimMontage "/Game/Player/AimationMontage/New/AttackCombo1/Combo_Attack_01_01_Seq_Montage.Combo_Attack_01_01_Seq_Montage" 1.0 "None"))
            (:1
              (Variables|Default|SetAttack%20Count 2)
              (Animation|PlayAnimMontage "/Game/Player/AimationMontage/New/AttackCombo1/Combo_Attack_01_02_Seq_Montage.Combo_Attack_01_02_Seq_Montage" 1.0 "None"))
            (:2
              (Variables|Default|SetAttack%20Count 3)
              (Animation|PlayAnimMontage "/Game/Player/AimationMontage/New/AttackCombo1/Combo_Attack_01_03_Seq_Montage.Combo_Attack_01_03_Seq_Montage" 1.0 "None"))
            (:3
              (Variables|Default|SetAttack%20Count 0)
              (Animation|PlayAnimMontage "/Game/Player/AimationMontage/New/AttackCombo1/Combo_Attack_01_04_Seq_Montage.Combo_Attack_01_04_Seq_Montage" 1.0 "None"))))
        (:1
          (switch int (Variables|Default|GetAttack%20Count)
            (:0
              (Variables|Default|SetAttack%20Count 1)
              (Animation|PlayAnimMontage "/Game/Player/AimationMontage/New/AttackCombo2/Combo_Attack_02_01_Seq_Montage.Combo_Attack_02_01_Seq_Montage" 1.0 "None"))
            (:1
              (Variables|Default|SetAttack%20Count 2)
              (Animation|PlayAnimMontage "/Game/Player/AimationMontage/New/AttackCombo2/Combo_Attack_02_02_Seq_Montage.Combo_Attack_02_02_Seq_Montage" 1.0 "None"))
            (:2
              (Variables|Default|SetAttack%20Count 3)
              (Animation|PlayAnimMontage "/Game/Player/AimationMontage/New/AttackCombo2/Combo_Attack_02_03_Seq_Montage.Combo_Attack_02_03_Seq_Montage" 1.0 "None"))
            (:3
              (Variables|Default|SetAttack%20Count 0)
              (Animation|PlayAnimMontage "/Game/Player/AimationMontage/New/AttackCombo2/Combo_Attack_02_04_Seq_Montage.Combo_Attack_02_04_Seq_Montage" 1.0 "None"))))
        (:2
          (switch int (Variables|Default|GetAttack%20Count)
            (:0
              (Variables|Default|SetAttack%20Count 1)
              (Animation|PlayAnimMontage "/Game/Player/AimationMontage/New/AttackCombo3/Combo_Attack_03_01_Seq_Montage.Combo_Attack_03_01_Seq_Montage" 1.0 "None"))
            (:1
              (Variables|Default|SetAttack%20Count 2)
              (Animation|PlayAnimMontage "/Game/Player/AimationMontage/New/AttackCombo3/Combo_Attack_03_02_Seq_Montage.Combo_Attack_03_02_Seq_Montage" 1.0 "None"))
            (:2
              (Variables|Default|SetAttack%20Count 3)
              (Animation|PlayAnimMontage "/Game/Player/AimationMontage/New/AttackCombo3/Combo_Attack_03_03_Seq_Montage.Combo_Attack_03_03_Seq_Montage" 1.0 "None"))
            (:3
              (Variables|Default|SetAttack%20Count 0)
              (Animation|PlayAnimMontage "/Game/Player/AimationMontage/New/AttackCombo3/Combo_Attack_03_04_Seq_Montage.Combo_Attack_03_04_Seq_Montage" 1.0 "None"))))
        (:3
          (switch int (Variables|Default|GetAttack%20Count)
            (:0
              (Variables|Default|SetAttack%20Count 1)
              (Animation|PlayAnimMontage "/Game/Player/AimationMontage/New/AttackCombo4/Combo_Attack_04_01_Seq_Montage.Combo_Attack_04_01_Seq_Montage" 1.0 "None"))
            (:1
              (Variables|Default|SetAttack%20Count 2)
              (Animation|PlayAnimMontage "/Game/Player/AimationMontage/New/AttackCombo4/Combo_Attack_04_02_Seq_Montage.Combo_Attack_04_02_Seq_Montage" 1.0 "None"))
            (:2
              (Variables|Default|SetAttack%20Count 3)
              (Animation|PlayAnimMontage "/Game/Player/AimationMontage/New/AttackCombo4/Combo_Attack_04_03_Seq_Montage.Combo_Attack_04_03_Seq_Montage" 1.0 "None"))
            (:3
              (Variables|Default|SetAttack%20Count 0)
              (Animation|PlayAnimMontage "/Game/Player/AimationMontage/New/AttackCombo4/Combo_Attack_04_04_Seq_Montage.Combo_Attack_04_04_Seq_Montage" 1.0 "None"))))))))

(event Custom|ResetCombo
  ;[1 1 1] Attack
  (Variables|Default|SetAttack%20Count 0)
  (Variables|Default|SetSave%20Attack false)
  (Variables|Default|SetIs%20Attacking false))

(event Input|EnhancedActionEvents|EnhancedInputActionIA_Attack
  (params (ActionValue :type Boolean) (ElapsedSeconds :type Float%20%28double-precision%29) (TriggeredSeconds :type Float%20%28double-precision%29) (InputAction :type Input%20Action%20Object%20Reference :default "/Game/Player/Inputs/GameInput/Actions/IA_Attack.IA_Attack"))
  ;[1 1 1] Attack
  (:Started
    (if (not (Math|Boolean|ORBoolean (Variables|Default|GetIsFalling) (Variables|Default|GetIs%20Rolling) (Variables|Default|GetIs%20Running)))
      (if (Variables|Default|GetIs%20Attacking)
        (Variables|Default|SetSave%20Attack true)
        (else
          (Variables|Default|SetIs%20Attacking true)
          (switch int (Variables|Default|GetAttack%20Type)
            (:0
              (switch int (Variables|Default|GetAttack%20Count)
                (:0
                  (Variables|Default|SetAttack%20Count 1)
                  (Animation|PlayAnimMontage "/Game/Player/AimationMontage/New/AttackCombo1/Combo_Attack_01_01_Seq_Montage.Combo_Attack_01_01_Seq_Montage" 1.0 "None"))
                (:1
                  (Variables|Default|SetAttack%20Count 2)
                  (Animation|PlayAnimMontage "/Game/Player/AimationMontage/New/AttackCombo1/Combo_Attack_01_02_Seq_Montage.Combo_Attack_01_02_Seq_Montage" 1.0 "None"))
                (:2
                  (Variables|Default|SetAttack%20Count 3)
                  (Animation|PlayAnimMontage "/Game/Player/AimationMontage/New/AttackCombo1/Combo_Attack_01_03_Seq_Montage.Combo_Attack_01_03_Seq_Montage" 1.0 "None"))
                (:3
                  (Variables|Default|SetAttack%20Count 0)
                  (Animation|PlayAnimMontage "/Game/Player/AimationMontage/New/AttackCombo1/Combo_Attack_01_04_Seq_Montage.Combo_Attack_01_04_Seq_Montage" 1.0 "None"))))
            (:1
              (switch int (Variables|Default|GetAttack%20Count)
                (:0
                  (Variables|Default|SetAttack%20Count 1)
                  (Animation|PlayAnimMontage "/Game/Player/AimationMontage/New/AttackCombo2/Combo_Attack_02_01_Seq_Montage.Combo_Attack_02_01_Seq_Montage" 1.0 "None"))
                (:1
                  (Variables|Default|SetAttack%20Count 2)
                  (Animation|PlayAnimMontage "/Game/Player/AimationMontage/New/AttackCombo2/Combo_Attack_02_02_Seq_Montage.Combo_Attack_02_02_Seq_Montage" 1.0 "None"))
                (:2
                  (Variables|Default|SetAttack%20Count 3)
                  (Animation|PlayAnimMontage "/Game/Player/AimationMontage/New/AttackCombo2/Combo_Attack_02_03_Seq_Montage.Combo_Attack_02_03_Seq_Montage" 1.0 "None"))
                (:3
                  (Variables|Default|SetAttack%20Count 0)
                  (Animation|PlayAnimMontage "/Game/Player/AimationMontage/New/AttackCombo2/Combo_Attack_02_04_Seq_Montage.Combo_Attack_02_04_Seq_Montage" 1.0 "None"))))
            (:2
              (switch int (Variables|Default|GetAttack%20Count)
                (:0
                  (Variables|Default|SetAttack%20Count 1)
                  (Animation|PlayAnimMontage "/Game/Player/AimationMontage/New/AttackCombo3/Combo_Attack_03_01_Seq_Montage.Combo_Attack_03_01_Seq_Montage" 1.0 "None"))
                (:1
                  (Variables|Default|SetAttack%20Count 2)
                  (Animation|PlayAnimMontage "/Game/Player/AimationMontage/New/AttackCombo3/Combo_Attack_03_02_Seq_Montage.Combo_Attack_03_02_Seq_Montage" 1.0 "None"))
                (:2
                  (Variables|Default|SetAttack%20Count 3)
                  (Animation|PlayAnimMontage "/Game/Player/AimationMontage/New/AttackCombo3/Combo_Attack_03_03_Seq_Montage.Combo_Attack_03_03_Seq_Montage" 1.0 "None"))
                (:3
                  (Variables|Default|SetAttack%20Count 0)
                  (Animation|PlayAnimMontage "/Game/Player/AimationMontage/New/AttackCombo3/Combo_Attack_03_04_Seq_Montage.Combo_Attack_03_04_Seq_Montage" 1.0 "None"))))
            (:3
              (switch int (Variables|Default|GetAttack%20Count)
                (:0
                  (Variables|Default|SetAttack%20Count 1)
                  (Animation|PlayAnimMontage "/Game/Player/AimationMontage/New/AttackCombo4/Combo_Attack_04_01_Seq_Montage.Combo_Attack_04_01_Seq_Montage" 1.0 "None"))
                (:1
                  (Variables|Default|SetAttack%20Count 2)
                  (Animation|PlayAnimMontage "/Game/Player/AimationMontage/New/AttackCombo4/Combo_Attack_04_02_Seq_Montage.Combo_Attack_04_02_Seq_Montage" 1.0 "None"))
                (:2
                  (Variables|Default|SetAttack%20Count 3)
                  (Animation|PlayAnimMontage "/Game/Player/AimationMontage/New/AttackCombo4/Combo_Attack_04_03_Seq_Montage.Combo_Attack_04_03_Seq_Montage" 1.0 "None"))
                (:3
                  (Variables|Default|SetAttack%20Count 0)
                  (Animation|PlayAnimMontage "/Game/Player/AimationMontage/New/AttackCombo4/Combo_Attack_04_04_Seq_Montage.Combo_Attack_04_04_Seq_Montage" 1.0 "None"))))))))))

(event Input|EnhancedActionEvents|EnhancedInputActionIA_Rolling
  (params (ActionValue :type Boolean) (ElapsedSeconds :type Float%20%28double-precision%29) (TriggeredSeconds :type Float%20%28double-precision%29) (InputAction :type Input%20Action%20Object%20Reference :default "/Game/Player/Inputs/GameInput/Actions/IA_Rolling.IA_Rolling"))
  ;[1 1 1] Roll
  (if (not (Variables|Default|GetIsFalling))
    (Utilities|FlowControl|DoOnce false :!label _label
      (:Completed
        (bind _newparam (CallFunction|Rolling))
        (Utilities|FlowControl|Delay _newparam)
        (Variables|Default|SetIs%20Rolling false)
        (goto _label Reset)))))

(event Input|EnhancedActionEvents|EnhancedInputActionIA_RunningMode
  (params (ActionValue :type Boolean) (ElapsedSeconds :type Float%20%28double-precision%29) (TriggeredSeconds :type Float%20%28double-precision%29) (InputAction :type Input%20Action%20Object%20Reference :default "/Game/Player/Inputs/GameInput/Actions/IA_RunningMode.IA_RunningMode"))
  (bind _charactermovement (Variables|Character|GetCharacterMovement))
  (bind _sword (Variables|컴포넌트|GetSword))
  ;[1 1 1] RunningMode
  (:Started
    (if (and (not (Variables|Default|GetIs%20Attacking)) (not (Variables|Default|GetisRolling)))
      (Utilities|FlowControl|DoOnce false :!label _label
        (:Completed
          (if (Variables|Default|GetIs%20Running)
            (Variables|Default|SetIs%20Running false)
            (Variables|/Script/Engine.CharacterMovementComponent|SetMaxWalkSpeed _charactermovement 5e+02)
            (bind _returnvalue (Animation|PlayAnimMontage "/Game/Player/AimationMontage/RunningMode_End_Montage.RunningMode_End_Montage" 1.0 "None"))
            (Utilities|FlowControl|Delay 0.4)
            (Rendering|SetVisibility _sword true false)
            (Utilities|FlowControl|Delay (- _returnvalue 0.4))
            (goto _label Reset)
            (else
              (Variables|Default|SetIs%20Running true)
              (Variables|/Script/Engine.CharacterMovementComponent|SetMaxWalkSpeed _charactermovement 7e+02)
              (bind _returnvalue_2 (Animation|PlayAnimMontage "/Game/Player/AimationMontage/RunningMode_Start_Montage.RunningMode_Start_Montage" 1.0 "None"))
              (Utilities|FlowControl|Delay _returnvalue_2)
              (Rendering|SetVisibility _sword false false)
              (goto _label Reset))))))))

(event Input|EnhancedActionEvents|EnhancedInputActionIA_Guard
  (params (ActionValue :type Boolean) (ElapsedSeconds :type Float%20%28double-precision%29) (TriggeredSeconds :type Float%20%28double-precision%29) (InputAction :type Input%20Action%20Object%20Reference :default "/Game/Player/Inputs/GameInput/Actions/IA_Guard.IA_Guard"))
  (:Started
    (Variables|Default|SetIs%20Blocking true))
  (:Completed
    (Variables|Default|SetIs%20Blocking false)))

(event EventBeginPlay)

(event Game|Damage|EventAnyDamage
  (params (Damage :type Float%20%28single-precision%29) (DamageType :type Damage%20Type%20Object%20Reference) (InstigatedBy :type Controller%20Object%20Reference) (DamageCauser :type Actor%20Object%20Reference))
  (CallFunction|DamageReaction DamageCauser))

(event EventTick
  (params (DeltaSeconds :type Float%20%28single-precision%29))
  (Variables|Default|SetIsFalling (AI|Components|NavMovement|IsFalling (Variables|Character|GetCharacterMovement)))
  (if (Variables|Default|GetIs%20Blocking)
    (CallFunction|DrawBlock)))

(event Input|KeyboardEvents|1
  (params (Key :type Key%20Structure :default "None"))
  ;[1 1 1] Attack
  (:Pressed
    (Variables|Default|SetAttack%20Type 0)
    (Development|PrintString "AttackCombo1")))

(event Input|KeyboardEvents|2
  (params (Key :type Key%20Structure :default "None"))
  ;[1 1 1] Attack
  (:Pressed
    (Variables|Default|SetAttack%20Type 1)
    (Development|PrintString "AttackCombo2")))

(event Input|KeyboardEvents|3
  (params (Key :type Key%20Structure :default "None"))
  ;[1 1 1] Attack
  (:Pressed
    (Variables|Default|SetAttack%20Type 2)
    (Development|PrintString "AttackCombo3")))

(event Input|KeyboardEvents|4
  (params (Key :type Key%20Structure :default "None"))
  ;[1 1 1] Attack
  (:Pressed
    (Variables|Default|SetAttack%20Type 3)
    (Development|PrintString "AttackCombo4")))

(fn ConstructionScript
  (Components|SkinnedMesh|SetLeaderPoseComponent (Variables|컴포넌트|GetFeet) (Variables|Character|GetMesh) false false))

(fn Rolling
  (Variables|Default|SetIs%20Rolling true)
  (if (> (Math|Vector2D|Vector2DLength (Input|EnhancedActionValues|GetIA_Move)) 0.0)
    (Transformation|SetActorRotation (Math|Conversions|RotationFromXVector (Class|Pawn|GetLastMovementInputVector)))
    (else
      (Transformation|SetActorRotation (Math|Conversions|RotationFromXVector (Transformation|GetActorForwardVector)))))
  (if (Variables|Default|GetIs%20Running)
    (bind _returnvalue (Animation|PlayAnimMontage "/Game/Player/AimationMontage/Roll_F_0_Seq_Montage.Roll_F_0_Seq_Montage" 1.0 "None"))
    (return (- _returnvalue 0.3))
    (else
      (bind _returnvalue_2 (Animation|PlayAnimMontage "/Game/Player/AimationMontage/New/Rolling/Roll_Combat_F_0_Seq_Montage.Roll_Combat_F_0_Seq_Montage" 1.0 "None"))
      (if (Variables|Default|GetIs%20Attacking)
        (CallFunction|ResetCombo))
      (return (- _returnvalue_2 0.3)))))

(fn TargetActorDegree
  (params (TargetActor :type Actor%20Object%20Reference))
  (bind _returnvalue (Transformation|GetActorLocation))
  (bind _returnvalue_2 (Transformation|GetActorForwardVector))
  (bind _returnvalue_3 (Transformation|GetActorLocation TargetActor))
  (bind _returnvalue_4 (Math|Vector|GetUnitDirection(Vector) _returnvalue _returnvalue_3))
  (bind _returnvalue_5 (Math|Vector|DotProduct _returnvalue_4 _returnvalue_2))
  (bind _returnvalue_6 (Math|Trig|Acos(Degrees) _returnvalue_5))
  (bind _returnvalue_7 (Math|Trig|RadiansToDegrees _returnvalue_6))
  (if (> (.y (Math|Vector|CrossProduct _returnvalue_4 (Transformation|GetActorRightVector))) 0.0)
    (return (- 3.6e+02 _returnvalue_7))
    (else
      (return _returnvalue_7))))

(fn DamageReaction
  (params (DamageCauser :type Actor%20Object%20Reference))
  (bind _returnvalue (Transformation|GetActorLocation))
  (bind _returnvalue_2 (Transformation|GetActorForwardVector))
  (bind _returnvalue_3 (Transformation|GetActorLocation DamageCauser))
  (bind _returnvalue_4 (Math|Vector|GetUnitDirection(Vector) _returnvalue _returnvalue_3))
  (bind _returnvalue_5 (Math|Vector|DotProduct _returnvalue_4 _returnvalue_2))
  (bind _returnvalue_6 (Math|Trig|Acos(Degrees) _returnvalue_5))
  (bind _returnvalue_7 (Math|Trig|RadiansToDegrees _returnvalue_6))
  (bind _returnvalue_8 (> _returnvalue_7 4e+01))
  (bind _returnvalue_9 (> _returnvalue_7 1.4e+02))
  (if (> (.y (Math|Vector|CrossProduct _returnvalue_4 (Transformation|GetActorRightVector))) 0.0)
    (if _returnvalue_8
      (if _returnvalue_9
        (Animation|PlayAnimMontage "/Game/Player/AimationMontage/Hit_Combat_B_Seq_Montage.Hit_Combat_B_Seq_Montage" 1.0 "None" :!label _label)
        (else
          (Animation|PlayAnimMontage "/Game/Player/AimationMontage/Hit_Combat_L_Seq_Montage.Hit_Combat_L_Seq_Montage" 1.0 "None")))
      (else
        (Animation|PlayAnimMontage "/Game/Player/AimationMontage/Hit_Combat_F_Seq_Montage.Hit_Combat_F_Seq_Montage" 1.0 "None" :!label _label_2)))
    (elif _returnvalue_8
      (if _returnvalue_9
        (goto _label)
        (else
          (Animation|PlayAnimMontage "/Game/Player/AimationMontage/Hit_Combat_R_Seq_Montage.Hit_Combat_R_Seq_Montage" 1.0 "None")))
      (else
        (goto _label_2)))))

(fn DrawBlock
  (bind _returnvalue (Transformation|GetActorLocation))
  (bind _returnvalue_2 (Transformation|GetActorForwardVector))
  (bind _length (LocalVariables|Getlength))
  (bind _returnvalue_3 (- (.z _returnvalue) 9e+01))
  (bind _returnvalue_4 (Math|Vector|MakeVector (.x _returnvalue) (.y _returnvalue) _returnvalue_3))
  (Class|KismetSystemLibrary|DrawDebugCylinder _returnvalue_4 _returnvalue_4 3e+02 24 "(R=1.000000,G=0.000000,B=0.000000,A=1.000000)" 0.0 2.0)
  (Rendering|Debug|DrawDebugLine _returnvalue_4 (+ (* (Math|Vector|RotateVector _returnvalue_2 "0.000000,45.000000,0.000000") _length) _returnvalue_4) "(R=1.000000,G=0.000000,B=0.000000,A=1.000000)" 0.0 2.0)
  (Rendering|Debug|DrawDebugLine _returnvalue_4 (+ _returnvalue_4 (* _length (Math|Vector|RotateVector _returnvalue_2 "0.000000,-45.000000,0.000000"))) "(R=1.000000,G=0.000000,B=0.000000,A=1.000000)" 0.0 3.0))