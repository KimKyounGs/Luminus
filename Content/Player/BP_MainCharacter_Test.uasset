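; Test player character for melee combat, with a four-montage combo, directional roll, run toggle, lock-on and modular body meshes following the main mesh.
; Clicks during attacks are buffered for AttackSave to chain the next forward-impulse swing, until ResetCombo clears it.
; AttackHitTrace toggles a looping timer that sphere-traces along the weapon and applies damage.
; Incoming damage only prints attacker yaw and name; game-instance loading logic is disconnected.
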(event Custom|AttackSave
  ;[1 1 1] Attack
  (if (not (Variables|Default|GetisFalling))
    (if (Variables|Default|GetSaveAttack)
      (Variables|Default|SetSaveAttack false)
      (Variables|/Script/Engine.CharacterMovementComponent|SetMaxWalkSpeed (Variables|Character|GetCharacterMovement) 0.0)
      (CallFunction|AttackMove 1e+03)
      (switch int (Variables|Default|GetAttackCount)
        (:0
          (Variables|Default|SetAttackCount 1)
          (Animation|PlayAnimMontage "/Game/Player/AimationMontage/Attack_A.Attack_A" 1.0 "None"))
        (:1
          (Variables|Default|SetAttackCount 2)
          (Animation|PlayAnimMontage "/Game/Player/AimationMontage/PrimaryAttack_B_Slow_Montage1.PrimaryAttack_B_Slow_Montage1" 1.0 "None"))
        (:2
          (Variables|Default|SetAttackCount 3)
          (Animation|PlayAnimMontage "/Game/Player/AimationMontage/PrimaryAttack_C_Slow_Montage1.PrimaryAttack_C_Slow_Montage1" 1.0 "None"))
        (:3
          (Variables|Default|SetAttackCount 0)
          (Animation|PlayAnimMontage "/Game/Player/AimationMontage/PrimaryAttack_D_Slow_Montage1.PrimaryAttack_D_Slow_Montage1" 1.0 "None"))))))

(event Custom|AttackHitTrace
  (params (TraceOn :type Boolean))
  ;[1 1 1] Hit Trace Start
  (if TraceOn
    (bind _returnvalue (Utilities|Time|SetTimerbyFunctionName 0 "Hit Trace" 0.01 true))
    (Variables|Default|SetAttackTraceTimerHandle _returnvalue)
    (else
      (Utilities|Time|ClearandInvalidateTimerbyHandle (Variables|Default|GetAttackTraceTimerHandle)))))

(event Custom|ResetCombo
  ;[1 1 1] Attack
  (Variables|Default|SetAttackCount 0)
  (Variables|Default|SetSaveAttack false)
  (Variables|Default|SetIsAttacking false)
  (Variables|/Script/Engine.CharacterMovementComponent|SetMaxWalkSpeed (Variables|Character|GetCharacterMovement) 5e+02))

(event Input|EnhancedActionEvents|EnhancedInputActionIA_Rolling
  (params (ActionValue :type Boolean) (ElapsedSeconds :type Float%20%28double-precision%29) (TriggeredSeconds :type Float%20%28double-precision%29) (InputAction :type Input%20Action%20Object%20Reference :default "/Game/Player/Inputs/GameInput/Actions/IA_Rolling.IA_Rolling"))
  ;[1 1 1] Rolling
  (if (not (Variables|Default|GetisFalling))
    (Utilities|FlowControl|DoOnce false :!label _label
      (:Completed
        (if (> (Math|Vector2D|Vector2DLength (Input|EnhancedActionValues|GetIA_Move)) 0.0)
          (bind _animlength (CallFunction|Rolling (Math|Conversions|RotationFromXVector (Class|Pawn|GetLastMovementInputVector))))
          (Utilities|FlowControl|Delay _animlength)
          (Variables|Default|SetisRolling false)
          (goto _label Reset)
          (else
            (bind _animlength_2 (CallFunction|Rolling (Pawn|GetControlRotation :!class /Script/Engine.Pawn)))
            (Utilities|FlowControl|Delay _animlength_2)
            (Variables|Default|SetisRolling false)
            (goto _label Reset)))))))

(event Input|EnhancedActionEvents|EnhancedInputActionIA_LockOn
  (params (ActionValue :type Boolean) (ElapsedSeconds :type Float%20%28double-precision%29) (TriggeredSeconds :type Float%20%28double-precision%29) (InputAction :type Input%20Action%20Object%20Reference :default "/Game/Player/Inputs/GameInput/Actions/IA_LockOn.IA_LockOn"))
  (Default|StartLockon (Variables|Default|GetBP_LockOnComponent)))

(event Input|EnhancedActionEvents|EnhancedInputActionIA_RunningMode
  (params (ActionValue :type Boolean) (ElapsedSeconds :type Float%20%28double-precision%29) (TriggeredSeconds :type Float%20%28double-precision%29) (InputAction :type Input%20Action%20Object%20Reference :default "/Game/Player/Inputs/GameInput/Actions/IA_RunningMode.IA_RunningMode"))
  (bind _charactermovement (Variables|Character|GetCharacterMovement))
  (if (and (not (Variables|Default|GetIsAttacking)) (not (Variables|Default|GetisRolling)))
    (Utilities|FlowControl|DoOnce false :!label _label
      (:Completed
        (if (Variables|Default|GetIsRuning)
          (Variables|Default|SetRunning%20End true)
          (Utilities|FlowControl|Delay 1.1)
          (Variables|Default|SetIsRuning false)
          (Variables|/Script/Engine.CharacterMovementComponent|SetMaxWalkSpeed _charactermovement 5e+02)
          (Variables|Default|SetRunning%20End false)
          (goto _label Reset)
          (else
            (Variables|/Script/Engine.CharacterMovementComponent|SetMaxWalkSpeed _charactermovement 7e+02)
            (Variables|Default|SetRunning%20Start true)
            (Utilities|FlowControl|Delay 1.1)
            (Variables|Default|SetIsRuning true)
            (Variables|Default|SetRunning%20Start false)
            (goto _label Reset)))))))

(event EventBeginPlay)

(event EventTick
  (params (DeltaSeconds :type Float%20%28single-precision%29))
  (Variables|Default|SetisFalling (AI|Components|NavMovement|IsFalling (Variables|Character|GetCharacterMovement))))

(event Game|Damage|EventAnyDamage
  (params (Damage :type Float%20%28single-precision%29) (DamageType :type Damage%20Type%20Object%20Reference) (InstigatedBy :type Controller%20Object%20Reference) (DamageCauser :type Actor%20Object%20Reference))
  (CallFunction|GetHitDirection DamageCauser)
  (Development|PrintString (Utilities|GetDisplayName DamageCauser)))

(event Input|MouseEvents|LeftMouseButton
  (params (Key :type Key%20Structure :default "None"))
  ;[1 1 1] Attack
  (:Pressed
    (if (Math|Boolean|ANDBoolean (not (Variables|Default|GetIsRuning)) (not (Variables|Default|GetisFalling)) (not (Variables|Default|GetisRolling)))
      (if (Variables|Default|GetIsAttacking)
        (Variables|Default|SetSaveAttack true)
        (else
          (Variables|Default|SetIsAttacking true)
          (Variables|/Script/Engine.CharacterMovementComponent|SetMaxWalkSpeed (Variables|Character|GetCharacterMovement) 0.0)
          (CallFunction|AttackMove 1e+03)
          (switch int (Variables|Default|GetAttackCount)
            (:0
              (Variables|Default|SetAttackCount 1)
              (Animation|PlayAnimMontage "/Game/Player/AimationMontage/Attack_A.Attack_A" 1.0 "None"))
            (:1
              (Variables|Default|SetAttackCount 2)
              (Animation|PlayAnimMontage "/Game/Player/AimationMontage/PrimaryAttack_B_Slow_Montage1.PrimaryAttack_B_Slow_Montage1" 1.0 "None"))
            (:2
              (Variables|Default|SetAttackCount 3)
              (Animation|PlayAnimMontage "/Game/Player/AimationMontage/PrimaryAttack_C_Slow_Montage1.PrimaryAttack_C_Slow_Montage1" 1.0 "None"))
            (:3
              (Variables|Default|SetAttackCount 0)
              (Animation|PlayAnimMontage "/Game/Player/AimationMontage/PrimaryAttack_D_Slow_Montage1.PrimaryAttack_D_Slow_Montage1" 1.0 "None"))))))))

(fn ConstructionScript
  (Components|SkinnedMesh|SetLeaderPoseComponent (Variables|Default|GetFeet) (Variables|Character|GetMesh) false false))

(fn AttackMove
  (params (Magniyude :type Float%20%28double-precision%29))
  (Physics|AddImpulse (Variables|Character|GetCharacterMovement) (* (Math|Vector|GetForwardVector (Variables|Default|GetCapsuleComponent)) Magniyude) true))

(fn HitTrace
  (bind _mesh (Variables|Character|GetMesh))
  (bind (_outhits _returnvalue) (Collision|MultiSphereTraceForObjects (Transformation|GetSocketLocation _mesh "FX_weapon_tip") (Transformation|GetSocketLocation _mesh "weapon_r") 1e+01 (Utilities|Array|MakeArray "ObjectTypeQuery3") false 0 "ForDuration"))
  (if _returnvalue
    (for _array_element _outhits
      (Game|Damage|ApplyDamage (.HitActor (Collision|BreakHitResult _array_element)) (Variables|Default|GetBase%20Damage) 0 0)
      (Development|PrintString (Utilities|GetDisplayName (.HitActor (Collision|BreakHitResult _array_element))))
      (Development|PrintString "Apply Damage로 데미지 냄"))))

(fn GetHitDirection
  (params (DamageCauser :type Actor%20Object%20Reference))
  (bind _output_get (Variables|Default|SetReturn%20Value%20Z%20%28Yaw%29 (.yaw (Math|Rotator|FindLookatRotation (Transformation|GetActorLocation) (Transformation|GetActorLocation DamageCauser)))))
  (Development|PrintString (Utilities|String|ToString(Float) _output_get)))

(fn Rolling
  (params (RotationOfRolling :type Rotator))
  (Variables|Default|SetisRolling true)
  (if (Variables|Default|GetIsAttacking)
    (Variables|Default|SetIsAttacking false)
    (Variables|/Script/Engine.CharacterMovementComponent|SetMaxWalkSpeed (Variables|Character|GetCharacterMovement) 5e+02))
  (Transformation|SetActorRotation RotationOfRolling)
  (bind _returnvalue (Animation|PlayAnimMontage "/Game/Player/AimationMontage/Roll_Montage.Roll_Montage" 1.0 "None"))
  (return (- _returnvalue 0.3)))

(fn GetHPPersent
  (return (/ (Variables|Default|GetMaxHealth) (Variables|Default|GetCurrentHealth))))