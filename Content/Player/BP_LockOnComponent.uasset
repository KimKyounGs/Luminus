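; Lock-on component for BP_MainCharacter that turns the camera toward a targeted pawn.
; StartLockOn sphere-traces pawns within LockOnRadius and picks the line-trace hit best aligned with camera forward by dot product.
; A looping timer interpolates control rotation toward the target, adjusts boom lag and offset, and releases beyond the radius.
; Retriggering switches to another centered target, filtered to one side by hit normal against camera right, or releases if none qualifies.
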(event Custom|StartLockOn
  (bind _newparam (CallFunction|LcokonTrace))
  (bind _charactereef (Variables|Default|GetCharacterEef))
  (bind _targettolockon (CallFunction|CheckforClosesTarget _newparam))
  (if (Variables|/Script/LuminusGame.LuminusGameCharacter|GetisLockOn _charactereef)
    (bind _target (CallFunction|SwitchTarget))
    (Utilities|IsValid _target
      (:Is%20Valid
        (Variables|Default|SetTargetLockedOn _target))
      (:Is%20Not%20Valid
        (CallFunction|StopTargetLockon)))
    (else
      (Utilities|IsValid _targettolockon
        (:Is%20Valid
          (Variables|/Script/LuminusGame.LuminusGameCharacter|SetisLockOn _charactereef true)
          (Variables|Default|SetTargetLockedOn _targettolockon)
          (bind _returnvalue (Utilities|Time|SetTimerbyEvent (delegate Custom|TargetLockOn) (Utilities|Time|GetWorldDeltaSeconds) true)))))))

(event Custom|TargetLockOn
  (bind _charactereef (Variables|Default|GetCharacterEef))
  (bind _cameraboom (Variables|/Script/LuminusGame.LuminusGameCharacter|GetCameraBoom _charactereef))
  (if (> (Math|Vector|Distance(Vector) (Transformation|GetActorLocation (Variables|Default|GetCharacterEef)) (Transformation|GetActorLocation (Variables|Default|GetTargetLockedOn))) (Variables|Default|GetLockOnRadius))
    (CallFunction|StopTargetLockon)
    (else
      (Pawn|SetControlRotation (Pawn|GetController _charactereef) (Math|Interpolation|RInterpTo (Class|SpringArmComponent|GetTargetRotation (Variables|/Script/LuminusGame.LuminusGameCharacter|GetCameraBoom _charactereef)) (Math|Rotator|FindLookatRotation (Transformation|GetWorldLocation (Variables|/Script/Engine.Actor|GetRootComponent (Variables|Default|GetCharacterEef))) (Transformation|GetActorLocation (Variables|Default|GetTargetLockedOn))) (Utilities|Time|GetWorldDeltaSeconds) 5.0))
      (Variables|/Script/Engine.SpringArmComponent|SetCameraRotationLagSpeed _cameraboom 1e+01)
      (Variables|/Script/Engine.SpringArmComponent|SetSocketOffset _cameraboom "0.000000,0.000000,100.000000"))))

(event Custom|Stop%20Target%20Lock%20On
  (bind _charactereef (Variables|Default|GetCharacterEef))
  (bind _cameraboom (Variables|/Script/LuminusGame.LuminusGameCharacter|GetCameraBoom _charactereef))
  (Utilities|Time|ClearandInvalidateTimerbyHandle (stale Custom|StartLockOn _returnvalue))
  (Variables|/Script/LuminusGame.LuminusGameCharacter|SetisLockOn _charactereef false)
  (Variables|/Script/Engine.SpringArmComponent|SetCameraRotationLagSpeed _cameraboom 0.0)
  (Variables|/Script/Engine.SpringArmComponent|SetSocketOffset _cameraboom "0, 0, 0")
  (Input|ResetIgnoreLookInput (Game|GetPlayerController 0)))

(event EventBeginPlay
  (bind _asbp_main_character (Utilities|Casting|CastToBP_MainCharacter (Game|GetPlayerCharacter 0)))
  (Variables|Default|SetCharacterEef _asbp_main_character))

(fn LcokonTrace
  (bind _charactereef (Variables|Default|GetCharacterEef))
  (bind _returnvalue (Transformation|GetActorLocation _charactereef))
  (bind (_outhits _returnvalue_2) (Collision|MultiSphereTraceForObjects _returnvalue _returnvalue (Variables|Default|GetLockOnRadius) (Utilities|Array|MakeArray "ObjectTypeQuery3") false 0 "None"))
  (if _returnvalue_2
    (for _array_element _outhits
      (Utilities|Array|Add (LocalVariables|GetLockOnTargets) (.HitActor (Collision|BreakHitResult _array_element))))
    (return (LocalVariables|GetLockOnTargets))))

(fn CheckforClosesTarget
  (params (Target :type Array%20of%20Actor%20Object%20References))
  (for _array_element Target
    (bind _returnvalue (Collision|LineTraceByChannel (Transformation|GetWorldLocation (Variables|/Script/LuminusGame.LuminusGameCharacter|GetFollowCamera (Variables|Default|GetCharacterEef))) (Transformation|GetActorLocation _array_element) "TraceTypeQuery2" false 0 "None"))
    (if _returnvalue
      (Math|Float|CompareFloat (CallFunction|CheckHowCloseTargetIstoCenter _array_element) (LocalVariables|GetLocalCompareFloat)
        (:>
          (LocalVariables|SetLocalCompareFloat (CallFunction|CheckHowCloseTargetIstoCenter _array_element))
          (LocalVariables|SetLocalTargetLockOn _array_element)))))
  (return (LocalVariables|GetLocalTargetLockOn)))

(fn CheckHowCloseTargetIstoCenter
  (params (Target :type Actor%20Object%20Reference))
  (bind _charactereef (Variables|Default|GetCharacterEef))
  ;[1 1 1] 카메라가 바라보는 것에서 얼마나 가까이 있는지 가까우면 1에 가까움
  (return (Math|Vector|DotProduct (Math|Vector|GetForwardVector (Variables|/Script/LuminusGame.LuminusGameCharacter|GetFollowCamera _charactereef)) (Math|Rotator|GetRotationXVector (Math|Rotator|FindLookatRotation (Transformation|GetActorLocation _charactereef) (Transformation|GetActorLocation Target))))))

(fn SwitchTarget
  (for _array_element (CallFunction|LcokonTrace)
    (bind (_outhit _returnvalue) (Collision|LineTraceForObjects (Transformation|GetWorldLocation (Variables|/Script/LuminusGame.LuminusGameCharacter|GetFollowCamera (Variables|Default|GetCharacterEef))) (Transformation|GetActorLocation _array_element) (Utilities|Array|MakeArray "ObjectTypeQuery3") false 0 "None"))
    (if _returnvalue
      (if (and (!= (Variables|Default|GetTargetLockedOn) _array_element) (< (Class|KismetMathLibrary|DegAsin (Math|Vector|DotProduct (Math|Vector|GetRightVector (Variables|/Script/LuminusGame.LuminusGameCharacter|GetFollowCamera (Variables|Default|GetCharacterEef))) (.Normal (Collision|BreakHitResult _outhit)))) 0.0))
        (Math|Float|CompareFloat (CallFunction|CheckHowCloseTargetIstoCenter _array_element) (LocalVariables|GetLocalTargetCompare)
          (:>
            (LocalVariables|SetLocalTargetCompare (CallFunction|CheckHowCloseTargetIstoCenter _array_element))
            (LocalVariables|SetLocalTargetTOLockOn _array_element))))))
  (return (LocalVariables|GetLocalTargetTOLockOn)))