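; BP_MainCharacter is the player character for melee combat, with combo attacks, a running mode, rolling and lock-on, and it triggers game loading on BeginPlay.
; Number keys pick one of four combo sets, and clicks during attacks are buffered until AttackSave chains the next montage.
; AttackHitTrace toggles a looping timer that sphere-traces along weapon sockets to apply damage.
; Incoming damage plays directional hit reactions without changing health.
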(event Custom|AttackSave
  (if (not (Variables|Default|GetisFalling))
    (if (Variables|Default|GetSaveAttack)
      (Variables|Default|SetSaveAttack false)
      (switch int (Variables|Default|GetAttackType)
        (:0
          (switch int (Variables|Default|GetAttackCount)
            (:0
              (Variables|Default|SetAttackCount 1)
              (Animation|PlayAnimMontage "/Game/Player/AimationMontage/New/AttackCombo1/Combo_Attack_01_01_Seq_Montage.Combo_Attack_01_01_Seq_Montage" 1.0 "None"))
            (:1
              (Variables|Default|SetAttackCount 2)
              (Animation|PlayAnimMontage 0 1.0 "None"))
            (:2
              (Variables|Default|SetAttackCount 3)
              (Animation|PlayAnimMontage 0 1.0 "None"))
            (:3
              (Variables|Default|SetAttackCount 0)
              (Animation|PlayAnimMontage 0 1.0 "None"))))
        (:1
          (switch int (Variables|Default|GetAttackCount)
            (:0
              (Variables|Default|SetAttackCount 1)
              (Animation|PlayAnimMontage 0 1.0 "None"))
            (:1
              (Variables|Default|SetAttackCount 2)
              (Animation|PlayAnimMontage 0 1.0 "None"))
            (:2
              (Variables|Default|SetAttackCount 3)
              (Animation|PlayAnimMontage 0 1.0 "None"))
            (:3
              (Variables|Default|SetAttackCount 0)
              (Animation|PlayAnimMontage 0 1.0 "None"))))
        (:2
          (switch int (Variables|Default|GetAttackCount)
            (:0
              (Variables|Default|SetAttackCount 1)
              (Animation|PlayAnimMontage 0 1.0 "None"))
            (:1
              (Variables|Default|SetAttackCount 2)
              (Animation|PlayAnimMontage 0 1.0 "None"))
            (:2
              (Variables|Default|SetAttackCount 3)
              (Animation|PlayAnimMontage 0 1.0 "None"))
            (:3
              (Variables|Default|SetAttackCount 0)
              (Animation|PlayAnimMontage 0 1.0 "None"))))
        (:3
          (switch int (Variables|Default|GetAttackCount)
            (:0
              (Variables|Default|SetAttackCount 1)
              (Animation|PlayAnimMontage 0 1.0 "None"))
            (:1
              (Variables|Default|SetAttackCount 2)
              (Animation|PlayAnimMontage 0 1.0 "None"))
            (:2
              (Variables|Default|SetAttackCount 3)
              (Animation|PlayAnimMontage 0 1.0 "None"))
            (:3
              (Variables|Default|SetAttackCount 0)
              (Animation|PlayAnimMontage 0 1.0 "None"))))))))

(event Custom|AttackHitTrace
  (params (TraceOn :type Boolean))
  ;[1 1 1] Hit Trace Start
  (if TraceOn
    (bind _returnvalue (Utilities|Time|SetTimerbyFunctionName 0 "Hit Trace" 0.01 true))
    (Variables|Default|SetAttackTraceTimerHandle _returnvalue)
    (else
      (Utilities|Time|ClearandInvalidateTimerbyHandle (Variables|Default|GetAttackTraceTimerHandle)))))

(event Custom|ResetCombo
  (Variables|Default|SetAttackCount 0)
  (Variables|Default|SetSaveAttack false)
  (Variables|Default|SetIsAttacking false))

(event Input|EnhancedActionEvents|EnhancedInputActionIA_Rolling
  (params (ActionValue :type Boolean) (ElapsedSeconds :type Float%20%28double-precision%29) (TriggeredSeconds :type Float%20%28double-precision%29) (InputAction :type Input%20Action%20Object%20Reference :default "/Game/Player/Inputs/GameInput/Actions/IA_Rolling.IA_Rolling"))
  ;[1 1 1] Rolling
  (if (not (Variables|Default|GetisFalling))
    (Utilities|FlowControl|DoOnce false :!label _label
      (:Completed
        (if (> (Math|Vector2D|Vector2DLength (Input|EnhancedActionValues|GetIA_Move)) 0.0)
          (bind _animlength (CallFunction|Rolling (Math|Conversions|RotationFromXVector (Class|Pawn|GetLastMovementInputVector))))
          (Utilities|FlowControl|Delay _animlength)
          (Variables|Default|SetisRolling false)
          (goto _label Reset)
          (else
            (bind _animlength_2 (CallFunction|Rolling (Pawn|GetControlRotation :!class /Script/Engine.Pawn)))
            (Utilities|FlowControl|Delay _animlength_2)
            (Variables|Default|SetisRolling false)
            (goto _label Reset)))))))

(event Input|EnhancedActionEvents|EnhancedInputActionIA_LockOn
  (params (ActionValue :type Boolean) (ElapsedSeconds :type Float%20%28double-precision%29) (TriggeredSeconds :type Float%20%28double-precision%29) (InputAction :type Input%20Action%20Object%20Reference :default "/Game/Player/Inputs/GameInput/Actions/IA_LockOn.IA_LockOn"))
  (Default|StartLockon (Variables|Default|GetBP_LockOnComponent)))

(event Input|EnhancedActionEvents|EnhancedInputActionIA_RunningMode
  (params (ActionValue :type Boolean) (ElapsedSeconds :type Float%20%28double-precision%29) (TriggeredSeconds :type Float%20%28double-precision%29) (InputAction :type Input%20Action%20Object%20Reference :default "/Game/Player/Inputs/GameInput/Actions/IA_RunningMode.IA_RunningMode"))
  (bind _charactermovement (Variables|Character|GetCharacterMovement))
  (if (and (not (Variables|Default|GetIsAttacking)) (not (Variables|Default|GetisRolling)))
    (Utilities|FlowControl|DoOnce false :!label _label
      (:Completed
        (if (Variables|Default|GetIsRuning)
          (Variables|Default|SetRunning%20End true)
          (Utilities|FlowControl|Delay 1.1)
          (Variables|Default|SetIsRuning false)
          (Variables|/Script/Engine.CharacterMovementComponent|SetMaxWalkSpeed _charactermovement 5e+02)
          (Variables|Default|SetRunning%20End false)
          (goto _label Reset)
          (else
            (Variables|/Script/Engine.CharacterMovementComponent|SetMaxWalkSpeed _charactermovement 7e+02)
            (Variables|Default|SetRunning%20Start true)
            (Utilities|FlowControl|Delay 1.1)
            (Variables|Default|SetIsRuning true)
            (Variables|Default|SetRunning%20Start false)
            (goto _label Reset)))))))

(event EventBeginPlay
  (Utilities|FlowControl|Sequence
    (:then_0
      (bind _aswb_my_game_instance (Utilities|Casting|CastToWB_MyGameInstance (Game|GetGameInstance)))
      (bind _output_get (Variables|Default|SetGameInstanceRef _aswb_my_game_instance))
      (Variables|/Game/Saving/WB_MyGameInstance.WB_MyGameInstance_C|SetPlayerCharacter _output_get self)
      (if (Variables|/Game/Saving/WB_MyGameInstance.WB_MyGameInstance_C|GetLoadGame? (Variables|Default|GetGameInstanceRef))
        (Default|GameLoad (Variables|Default|GetGameInstanceRef))
        (Default|LoadGame (Variables|Default|GetGameInstanceRef))
        (Variables|/Game/Saving/WB_MyGameInstance.WB_MyGameInstance_C|SetLoadGame? (Variables|Default|GetGameInstanceRef) false)))))

(event EventTick
  (params (DeltaSeconds :type Float%20%28single-precision%29))
  (Variables|Default|SetisFalling (AI|Components|NavMovement|IsFalling (Variables|Character|GetCharacterMovement))))

(event Game|Damage|EventAnyDamage
  (params (Damage :type Float%20%28single-precision%29) (DamageType :type Damage%20Type%20Object%20Reference) (InstigatedBy :type Controller%20Object%20Reference) (DamageCauser :type Actor%20Object%20Reference))
  (CallFunction|GetHitRection DamageCauser))

(event Input|MouseEvents|LeftMouseButton
  (params (Key :type Key%20Structure :default "None"))
  (:Pressed
    (if (Math|Boolean|ANDBoolean (not (Variables|Default|GetIsRuning)) (not (Variables|Default|GetisFalling)) (not (Variables|Default|GetisRolling)))
      (if (Variables|Default|GetIsAttacking)
        (Variables|Default|SetSaveAttack true)
        (else
          (Variables|Default|SetIsAttacking true)
          (switch int (Variables|Default|GetAttackType)
            (:0
              (switch int (Variables|Default|GetAttackCount)
                (:0
                  (Variables|Default|SetAttackCount 1)
                  (Animation|PlayAnimMontage "/Game/Player/AimationMontage/New/AttackCombo1/Combo_Attack_01_01_Seq_Montage.Combo_Attack_01_01_Seq_Montage" 1.0 "None"))
                (:1
                  (Variables|Default|SetAttackCount 2)
                  (Animation|PlayAnimMontage 0 1.0 "None"))
                (:2
                  (Variables|Default|SetAttackCount 3)
                  (Animation|PlayAnimMontage 0 1.0 "None"))
                (:3
                  (Variables|Default|SetAttackCount 0)
                  (Animation|PlayAnimMontage 0 1.0 "None"))))
            (:1
              (switch int (Variables|Default|GetAttackCount)
                (:0
                  (Variables|Default|SetAttackCount 1)
                  (Animation|PlayAnimMontage 0 1.0 "None"))
                (:1
                  (Variables|Default|SetAttackCount 2)
                  (Animation|PlayAnimMontage 0 1.0 "None"))
                (:2
                  (Variables|Default|SetAttackCount 3)
                  (Animation|PlayAnimMontage 0 1.0 "None"))
                (:3
                  (Variables|Default|SetAttackCount 0)
                  (Animation|PlayAnimMontage 0 1.0 "None"))))
            (:2
              (switch int (Variables|Default|GetAttackCount)
                (:0
                  (Variables|Default|SetAttackCount 1)
                  (Animation|PlayAnimMontage 0 1.0 "None"))
                (:1
                  (Variables|Default|SetAttackCount 2)
                  (Animation|PlayAnimMontage 0 1.0 "None"))
                (:2
                  (Variables|Default|SetAttackCount 3)
                  (Animation|PlayAnimMontage 0 1.0 "None"))
                (:3
                  (Variables|Default|SetAttackCount 0)
                  (Animation|PlayAnimMontage 0 1.0 "None"))))
            (:3
              (switch int (Variables|Default|GetAttackCount)
                (:0
                  (Variables|Default|SetAttackCount 1)
                  (Animation|PlayAnimMontage 0 1.0 "None"))
                (:1
                  (Variables|Default|SetAttackCount 2)
                  (Animation|PlayAnimMontage 0 1.0 "None"))
                (:2
                  (Variables|Default|SetAttackCount 3)
                  (Animation|PlayAnimMontage 0 1.0 "None"))
                (:3
                  (Variables|Default|SetAttackCount 0)
                  (Animation|PlayAnimMontage 0 1.0 "None"))))))))))

(event Input|KeyboardEvents|1
  (params (Key :type Key%20Structure :default "None"))
  (:Pressed
    (Variables|Default|SetAttackType 0)
    (Development|PrintString "AttackCombo1")))

(event Input|KeyboardEvents|2
  (params (Key :type Key%20Structure :default "None"))
  (:Pressed
    (Variables|Default|SetAttackType 1)
    (Development|PrintString "AttackCombo2")))

(event Input|KeyboardEvents|3
  (params (Key :type Key%20Structure :default "None"))
  (:Pressed
    (Variables|Default|SetAttackType 2)
    (Development|PrintString "AttackCombo3")))

(event Input|KeyboardEvents|4
  (params (Key :type Key%20Structure :default "None"))
  (:Pressed
    (Variables|Default|SetAttackType 3)
    (Development|PrintString "AttackCombo4")))

(fn ConstructionScript)

(fn AttackMove
  (params (Magniyude :type Float%20%28double-precision%29))
  (Physics|AddImpulse (Variables|Character|GetCharacterMovement) (* (Math|Vector|GetForwardVector (Variables|Default|GetCapsuleComponent)) Magniyude) true))

(fn HitTrace
  (bind _mesh (Variables|Character|GetMesh))
  (bind (_outhits _returnvalue) (Collision|MultiSphereTraceForObjects (Transformation|GetSocketLocation _mesh "FX_weapon_tip") (Transformation|GetSocketLocation _mesh "weapon_r") 1e+01 (Utilities|Array|MakeArray "ObjectTypeQuery3") false 0 "ForDuration"))
  (if _returnvalue
    (for _array_element _outhits
      (Game|Damage|ApplyDamage (.HitActor (Collision|BreakHitResult _array_element)) (Variables|Default|GetBase%20Damage) 0 0)
      (Development|PrintString (Utilities|GetDisplayName (.HitActor (Collision|BreakHitResult _array_element)))))))

(fn GetHitRection
  (params (DamageCauser :type Actor%20Object%20Reference))
  (bind _returnvalue (Transformation|GetActorLocation))
  (bind _returnvalue_2 (Transformation|GetActorForwardVector))
  (bind _returnvalue_3 (Transformation|GetActorLocation DamageCauser))
  (bind _returnvalue_4 (Math|Vector|GetUnitDirection(Vector) _returnvalue _returnvalue_3))
  (bind _returnvalue_5 (Math|Vector|DotProduct _returnvalue_4 _returnvalue_2))
  (bind _returnvalue_6 (Math|Trig|Acos(Degrees) _returnvalue_5))
  (bind _returnvalue_7 (Math|Trig|RadiansToDegrees _returnvalue_6))
  (if (> _returnvalue_7 5e+01)
    (if (> _returnvalue_7 1.2e+02)
      (Animation|PlayAnimMontage "/Game/Player/AimationMontage/Hitreact_Bwd_Montage.Hitreact_Bwd_Montage" 1.0 "None")
      (elif (> 9e+01 (Math|Trig|RadiansToDegrees (Math|Trig|Acos(Degrees) (Math|Vector|DotProduct _returnvalue_4 (Transformation|GetActorRightVector)))))
        (Animation|PlayAnimMontage "/Game/Player/AimationMontage/Hitreact_Right_Montage.Hitreact_Right_Montage" 1.0 "None")
        (else
          (Animation|PlayAnimMontage "/Game/Player/AimationMontage/Hitreact_Left_Montage.Hitreact_Left_Montage" 1.0 "None"))))
    (else
      (Animation|PlayAnimMontage "/Game/Player/AimationMontage/Hitreact_Fwd_Montage.Hitreact_Fwd_Montage" 1.0 "None"))))

(fn Rolling
  (params (RotationOfRolling :type Rotator))
  (Variables|Default|SetisRolling true)
  (if (Variables|Default|GetIsAttacking)
    (Variables|Default|SetIsAttacking false)
    (Variables|/Script/Engine.CharacterMovementComponent|SetMaxWalkSpeed (Variables|Character|GetCharacterMovement) 5e+02))
  (Transformation|SetActorRotation RotationOfRolling)
  (bind _returnvalue (Animation|PlayAnimMontage "/Game/Player/AimationMontage/Roll_Montage.Roll_Montage" 1.0 "None"))
  (return (- _returnvalue 0.3)))

(fn GetHPPersent
  (return (/ (Variables|Default|GetCurrentHealth) (Variables|Default|GetMaxHealth))))