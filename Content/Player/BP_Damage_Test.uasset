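; BP_Damage_Test is a test actor that deals repeated damage to a player character that overlaps it.
; Begin overlap caches the actor as either BP_MainCharacter or BP_Character.
; Tick damages the cached character, preferring BP_MainCharacter, using a DoOnce reset by a Delay to hit once per second.
; The references are never cleared, so damage continues after overlap ends while the character remains valid.
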(event EventBeginPlay)

(event Collision|EventActorBeginOverlap
  (params (OtherActor :type Actor%20Object%20Reference))
  (bind _asbp_main_character (Utilities|Casting|CastToBP_MainCharacter OtherActor)
    (:then
      (Variables|Default|SetAs%20BP%20Main%20Character _asbp_main_character))
    (:CastFailed
      (bind _asbp_character (Utilities|Casting|CastToBP_Character OtherActor))
      (Variables|Default|SetAs%20BP%20Character _asbp_character))))

(event EventTick
  (params (DeltaSeconds :type Float%20%28single-precision%29))
  (bind _as_bp_character (Variables|Default|GetAs%20BP%20Character))
  (bind _as_bp_main_character (Variables|Default|GetAs%20BP%20Main%20Character))
  (Utilities|IsValid _as_bp_main_character
    (:Is%20Valid
      (Utilities|FlowControl|DoOnce false :!label _label
        (:Completed
          (Game|Damage|ApplyDamage _as_bp_main_character 1e+01 0 self)
          (Utilities|FlowControl|Delay 1.0)
          (goto _label Reset))))
    (:Is%20Not%20Valid
      (Utilities|IsValid _as_bp_character
        (:Is%20Valid
          (Utilities|FlowControl|DoOnce false :!label _label_2
            (:Completed
              (Game|Damage|ApplyDamage _as_bp_character 1e+01 0 self)
              (Utilities|FlowControl|Delay 1.0)
              (goto _label_2 Reset))))))))

(fn ConstructionScript)